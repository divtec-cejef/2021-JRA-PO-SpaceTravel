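; BP_Arrow is a child-actor arrow that points toward the current objective, or a default objective when that one is invalid.
; Each Tick it aims its mesh with a look-at rotation, taking roll from the parent actor plus a 90-degree offset.
; It also polls whether the player spaceship's body overlaps the current asteroid checkpoint's box, teleporting the ship to that checkpoint's respawn point with the checkpoint's rotation.
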(event `self.ReceiveTick`
  (params (DeltaSeconds :type "Float (single-precision)"))
  (bind _mesh_arrow (`self.mesh_Arrow`))
  (bind _returnvalue_roll (`KismetMathLibrary.BreakRotator` (`self.K2_GetActorRotation` (`self.GetParentActor`))))
  (bind _returnvalue_roll_2 (`KismetMathLibrary.BreakRotator` (`self.K2_GetActorRotation` (`self.GetParentActor`))))
  (bind _output (`|GetArrayItem` (`self.Objectives`) (`self.currentObjectiveIndex`)))
  (`/Engine/EditorBlueprintResources/StandardMacros.IsValid` _output
    (:`Is Valid`
      (`SceneComponent.K2_SetWorldRotation` _mesh_arrow (`KismetMathLibrary.MakeRotator` (+ _returnvalue_roll_2 90.0) (.pitch (`KismetMathLibrary.FindLookAtRotation` (`SceneComponent.K2_GetComponentLocation` _mesh_arrow) (`self.K2_GetActorLocation` _output))) (.yaw (`KismetMathLibrary.FindLookAtRotation` (`SceneComponent.K2_GetComponentLocation` _mesh_arrow) (`self.K2_GetActorLocation` _output)))) false false)
      (bind _asbp_spaceship (cast `/Game/Blueprint/Spaceship/BP_Spaceship` (`GameplayStatics.GetPlayerPawn` 0)))
      (bind _asbp_asteroid_check_point (cast `/Game/Blueprint/Asteroides/BP_AsteroidCheckPoint` _output))
      (if (`PrimitiveComponent.IsOverlappingComponent` (`/Game/Blueprint/Spaceship/BP_Spaceship.SM_SpaceFighterGR2_Body` _asbp_spaceship) (`/Game/Blueprint/Asteroides/BP_AsteroidCheckPoint.Box` _asbp_asteroid_check_point))
        (`self.K2_TeleportTo` _asbp_spaceship (`SceneComponent.K2_GetComponentLocation` (`/Game/Blueprint/Asteroides/BP_AsteroidCheckPoint.RespawnPoint` _asbp_asteroid_check_point)) (`self.K2_GetActorRotation` _output))))
    (:`Is Not Valid`
      (`SceneComponent.K2_SetWorldRotation` _mesh_arrow (`KismetMathLibrary.MakeRotator` (+ _returnvalue_roll 90.0) (.pitch (`KismetMathLibrary.FindLookAtRotation` (`SceneComponent.K2_GetComponentLocation` _mesh_arrow) (`self.K2_GetActorLocation` (`self.DefaultObjective`)))) (.yaw (`KismetMathLibrary.FindLookAtRotation` (`SceneComponent.K2_GetComponentLocation` _mesh_arrow) (`self.K2_GetActorLocation` (`self.DefaultObjective`))))) false false))))

(fn `UserConstructionScript`)