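; BP_LazerPrimary is a ship component that acts as the primary laser weapon.
; Its Fire event spawns a BP_LazerProjectile at the actor's location and rotation, passing in the weapon's damage, speed, physics force, visual settings and parent ship.
; It then plays a firing sound and attaches a scaled muzzle flash to its Arrow, tinted to the laser color through particle parameters.
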(event `Fire`
  (bind _returnvalue (`self.K2_GetActorLocation`))
  (bind (_r _g _b) (break `LinearColor` (`self.Lazer_Primary_Color`)))
  (`|SpawnActorFromClass` "/Game/Blueprint/ShipComponents/BP_LazerProjectile.BP_LazerProjectile_C" (`KismetMathLibrary.MakeTransform` _returnvalue (`self.K2_GetActorRotation`) (`KismetMathLibrary.Conv_DoubleToVector` (`self.Lazer_Primary_Scale`))) "Undefined" "OverrideRootScale" null (`self.Lazer_Primary_Color`) (`self.Lazer_Primary_PhysicsForce`) (`self.Lazer_Primary_ExplosionScale`) (`self.ParentShip`) (`self.Lazer_Primary_DamageToApply`) (`self.Lazer_Primary_PhysicsForce_Multiplier_ForShield`) (`self.Lazer_Primary_Speed`) (`self.Lazer_Primary_ExplosionBrightness`) (`self.Lazer_Primary_PointLightBrightness`) (`self.Lazer_Primary_PointLightEnabled`) (`self.Lazer_Primary_MaterialGlowIntensity`) self)
  (`GameplayStatics.PlaySoundAtLocation` (`self.Lazer_Primary_SoundCue`) _returnvalue (struct) 1.0 1.0 0.0 null null null)
  (bind _returnvalue_2 (`GameplayStatics.SpawnEmitterAttached` "/Game/Particles/Spaceship/P_GR2_MuzzleFlash.P_GR2_MuzzleFlash" (`self.Arrow`) "None")) ; this is in local space
  (`SceneComponent.SetWorldScale3D` _returnvalue_2 (`KismetMathLibrary.Conv_DoubleToVector` (`self.MuzzleFlash_Scale`)))
  (`ParticleSystemComponent.SetFloatParameter` _returnvalue_2 "Color_R" _r)
  (`ParticleSystemComponent.SetFloatParameter` _returnvalue_2 "Color_G" _g)
  (`ParticleSystemComponent.SetFloatParameter` _returnvalue_2 "Color_B" _b))

(fn `UserConstructionScript`)