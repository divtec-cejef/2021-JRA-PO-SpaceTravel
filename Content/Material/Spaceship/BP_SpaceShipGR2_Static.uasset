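; Static, non-drivable GR2 space fighter prop, configured entirely in the construction script from exposed variables.
; It darkens the cockpit glass, optionally disables body collision, rotates the canopy by an open amount and retracts landing gear when not down.
; Dynamic material instances apply paint, roughness and cockpit glow to hull and joystick.
; Thruster glow and color drive flare materials, hull emission, point lights and square-root-eased flare mesh scale.
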(fn `UserConstructionScript`
  (bind _thruster_glow (`self.Thruster_Glow`))
  (bind _hull_material (`self.Hull_Material`))
  (bind _pointlight_thruster_l (`self.PointLight_Thruster_L`))
  (bind _sm_rocketflare_l (`self.SM_RocketFlare_L`))
  (bind _rocketflare_mat_0 (`self.RocketFlare_Mat_0`))
  (bind _sm_spacefightergr2_body (`self.SM_SpaceFighterGR2_Body`))
  (bind _hull_material_2 (`self.Hull_Material`))
  (bind _cockpit_glow_amount (`self.Cockpit_Glow_Amount`))
  (bind _sm_spacefighter_gr2_glass (`self.SM_SpaceFighter_GR2_Glass`))
  (`PrimitiveComponent.SetMaterial` _sm_spacefighter_gr2_glass 2 (`PrimitiveComponent.GetMaterial` _sm_spacefighter_gr2_glass 1)) ; Make inside of Glass Dark (Because it looks better from the outside and we wont be driving this ship)
  (if (not (`self.Collision`))
    (`PrimitiveComponent.SetCollisionEnabled` (`self.SM_SpaceFighterGR2_Body`) "NoCollision"))
  (bind _returnvalue (`PrimitiveComponent.CreateDynamicMaterialInstance` _sm_spacefightergr2_body 0 "/Game/Material/Spaceship/MI_SpaceFighter_GR2.MI_SpaceFighter_GR2" "None"))
  (bind _output_get (set `self.Hull_Material` _returnvalue))
  (`PrimitiveComponent.SetMaterial` _sm_spacefightergr2_body 0 _output_get)
  (bind _returnvalue_2 (`KismetMaterialLibrary.CreateDynamicMaterialInstance` "/Game/Material/Spaceship/MI_SpaceFighter_GR2_Joystick.MI_SpaceFighter_GR2_Joystick"))
  (bind _output_get_2 (set `self.Joystick_Material` _returnvalue_2))
  (`PrimitiveComponent.SetMaterial` (`self.SM_SpaceFighter_GR2_Joystick`) 0 _output_get_2)
  (`MaterialInstanceDynamic.SetVectorParameterValue` _hull_material_2 "Dif_Color_1" (`self.Paint_Color1`))
  (`MaterialInstanceDynamic.SetVectorParameterValue` _hull_material_2 "Dif_Color_2" (`self.Paint_Color2`))
  (`MaterialInstanceDynamic.SetScalarParameterValue` _hull_material_2 "Metal_Color_1" (`self.Paint_Metallic_1`))
  (`MaterialInstanceDynamic.SetScalarParameterValue` _hull_material_2 "Metal_Color_2" (`self.Paint_Metallic_2`))
  (`MaterialInstanceDynamic.SetScalarParameterValue` _hull_material_2 "Dif_Non-Color_Brightness" (`self.NonPainted_Brightness`))
  (`MaterialInstanceDynamic.SetScalarParameterValue` (`self.Joystick_Material`) "Dif_Non-Color_Brightness" (`self.NonPainted_Brightness`))
  (`MaterialInstanceDynamic.SetScalarParameterValue` _hull_material_2 "Dif_Color_1_Brightness" (`self.Paint_1_Brightness`))
  (`MaterialInstanceDynamic.SetScalarParameterValue` _hull_material_2 "Dif_Color_2_Brightness" (`self.Paint_2_Brightness`))
  (`MaterialInstanceDynamic.SetScalarParameterValue` _hull_material_2 "Rough_Color_1" (`self.Paint_Roughness_1`))
  (`MaterialInstanceDynamic.SetScalarParameterValue` _hull_material_2 "Rough_Color_2" (`self.Paint_Roughness_2`))
  (`MaterialInstanceDynamic.SetScalarParameterValue` _hull_material_2 "Roughness_Non-Color" (`self.NonPainted_Roughness`))
  (`MaterialInstanceDynamic.SetScalarParameterValue` _hull_material_2 "Thrust_On?" 0.0)
  (`MaterialInstanceDynamic.SetScalarParameterValue` _hull_material_2 "GlowBaked_Multiply" _cockpit_glow_amount)
  (`MaterialInstanceDynamic.SetScalarParameterValue` (`self.Joystick_Material`) "DiffuseGlow" (/ _cockpit_glow_amount 3.0))
  (`MaterialInstanceDynamic.SetScalarParameterValue` _hull_material_2 "GlowBaked_Source_Intensity" (`self.Cockpit_Glow_Highlights_Amount`))
  (`SceneComponent.K2_SetRelativeRotation` (`self.SM_SpaceFighter_GR2_Glass`) (`KismetMathLibrary.MakeRotator` 0.0 (`KismetMathLibrary.Lerp` 0.0 90.0 (`self.Glass_Door_Open?`))) false false) ; Rotate Canopy Glass
  (bind _returnvalue_3 (`KismetMaterialLibrary.CreateDynamicMaterialInstance` "/Game/Material/RocketFlare/MI_RocketFlare_0.MI_RocketFlare_0"))
  (bind _output_get_3 (set `self.RocketFlare_Mat_0` _returnvalue_3))
  (`PrimitiveComponent.SetMaterial` _sm_rocketflare_l 0 _output_get_3)
  (`PrimitiveComponent.SetMaterial` (`self.SM_RocketFlare_R`) 0 _output_get_3)
  (bind _returnvalue_4 (`KismetMaterialLibrary.CreateDynamicMaterialInstance` "/Game/Material/RocketFlare/MI_RocketFlare_1.MI_RocketFlare_1"))
  (bind _output_get_4 (set `self.RocketFlare_Mat_1` _returnvalue_4))
  (`PrimitiveComponent.SetMaterial` (`self.SM_RocketFlare_R`) 1 _output_get_4)
  (`PrimitiveComponent.SetMaterial` _sm_rocketflare_l 1 _output_get_4)
  (bind _returnvalue_5 (`KismetMaterialLibrary.CreateDynamicMaterialInstance` "/Game/Material/RocketFlare/MI_RocketFlare_2.MI_RocketFlare_2"))
  (bind _output_get_5 (set `self.RocketFlare_Mat_2` _returnvalue_5))
  (`PrimitiveComponent.SetMaterial` _sm_rocketflare_l 2 _output_get_5)
  (`PrimitiveComponent.SetMaterial` (`self.SM_RocketFlare_R`) 2 _output_get_5)
  (bind _returnvalue_6 (`KismetMaterialLibrary.CreateDynamicMaterialInstance` "/Game/Material/RocketFlare/MI_RocketFlare_3.MI_RocketFlare_3"))
  (bind _output_get_6 (set `self.RocketFlare_Mat_3` _returnvalue_6))
  (`PrimitiveComponent.SetMaterial` _sm_rocketflare_l 3 _output_get_6)
  (`PrimitiveComponent.SetMaterial` (`self.SM_RocketFlare_R`) 3 _output_get_6)
  (`MaterialInstanceDynamic.SetScalarParameterValue` _rocketflare_mat_0 "Opacity" (`self.Thruster_Glow`))
  (`MaterialInstanceDynamic.SetScalarParameterValue` (`self.RocketFlare_Mat_3`) "Opacity" (`self.Thruster_Glow`))
  (`MaterialInstanceDynamic.SetScalarParameterValue` (`self.RocketFlare_Mat_2`) "Opacity" (`self.Thruster_Glow`))
  (`MaterialInstanceDynamic.SetScalarParameterValue` (`self.RocketFlare_Mat_1`) "Opacity" (`self.Thruster_Glow`))
  (`MaterialInstanceDynamic.SetVectorParameterValue` _rocketflare_mat_0 "Color" (`self.Thruster_Color`))
  (`MaterialInstanceDynamic.SetVectorParameterValue` (`self.RocketFlare_Mat_1`) "Color" (`self.Thruster_Color`))
  (`MaterialInstanceDynamic.SetVectorParameterValue` (`self.RocketFlare_Mat_2`) "Color" (`self.Thruster_Color`))
  (`MaterialInstanceDynamic.SetVectorParameterValue` (`self.RocketFlare_Mat_3`) "Color" (`self.Thruster_Color`))
  (`MaterialInstanceDynamic.SetScalarParameterValue` _hull_material "Thrust_On?" _thruster_glow)
  (`MaterialInstanceDynamic.SetVectorParameterValue` _hull_material "FlareColor" (`self.Thruster_Color`))
  (`LightComponent.SetIntensity` _pointlight_thruster_l (`KismetMathLibrary.Lerp` 0.0 6500.0 _thruster_glow))
  (`LightComponent.SetIntensity` (`self.PointLight_Thruster_R`) (`KismetMathLibrary.Lerp` 0.0 6500.0 _thruster_glow))
  (`LightComponent.SetLightColor` _pointlight_thruster_l (`self.Thruster_Color`) true)
  (`LightComponent.SetLightColor` (`self.PointLight_Thruster_R`) (`self.Thruster_Color`) true)
  (`SceneComponent.SetRelativeScale3D` (`self.SM_RocketFlare_L`) (`KismetMathLibrary.VLerp` (0.01 1.0 1.0) (1.0 1.0 1.0) (`KismetMathLibrary.Sqrt` (`self.Thruster_Glow`))))
  (`SceneComponent.SetRelativeScale3D` (`self.SM_RocketFlare_R`) (`KismetMathLibrary.VLerp` (0.01 1.0 1.0) (1.0 1.0 1.0) (`KismetMathLibrary.Sqrt` (`self.Thruster_Glow`))))
  (if (not (`self.LandingGearDown`))
    (`SceneComponent.K2_SetRelativeLocation` (`self.SM_SpaceFighter_GR2_LGear_Front`) (397.100006 0.0 95.099998) false false)
    (`SceneComponent.K2_SetRelativeRotation` (`self.SM_SpaceFighter_GR2_LGear_Left`) (struct :`Roll` -90.0) false false)
    (`SceneComponent.K2_SetRelativeRotation` (`self.SM_SpaceFighter_GR2_LGear_Right`) (struct :`Roll` 90.0) false false)))