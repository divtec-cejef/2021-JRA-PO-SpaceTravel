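; BP_AsteroidCheckPoint is a station checkpoint in a chain of objectives for the player's spaceship.
; When a BP_Spaceship overlaps its sphere, it increments the objective index on the ship's BP_Arrow child actor and makes that next checkpoint's mesh visible.
; A Triggered flag stops a checkpoint from advancing the chain again once the next one is revealed.
; The construction script picks its mesh at random from StationMeshes.
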(event `self.ReceiveActorBeginOverlap`
  (params (OtherActor :type "Actor Object Reference"))
  (if (and (== (`GameplayStatics.GetObjectClass` OtherActor) "/Game/Blueprint/Spaceship/BP_Spaceship.BP_Spaceship_C") (`PrimitiveComponent.IsOverlappingActor` (`self.Sphere`) OtherActor))
    (bind _asbp_spaceship (cast `/Game/Blueprint/Spaceship/BP_Spaceship` OtherActor))
    (bind _asbp_arrow (cast `/Game/Blueprint/Spaceship/BP_Arrow` (`ChildActorComponent.ChildActor` (`/Game/Blueprint/Spaceship/BP_Spaceship.BP_Arrow` _asbp_spaceship))))
    (if (not (`self.Triggered`))
      (bind _result (`/Engine/EditorBlueprintResources/StandardMacros.IncrementInt` (`/Game/Blueprint/Spaceship/BP_Arrow.currentObjectiveIndex` _asbp_arrow))
        (:`  `
          (bind _asbp_asteroid_check_point (cast `/Game/Blueprint/Asteroides/BP_AsteroidCheckPoint` (`|GetArrayItem` (`/Game/Blueprint/Spaceship/BP_Arrow.Objectives` _asbp_arrow) _result)))
          (`SceneComponent.SetVisibility` (`/Game/Blueprint/Asteroides/BP_AsteroidCheckPoint.StaticMesh` _asbp_asteroid_check_point) true false)
          (set `self.Triggered` true))))))

(fn `UserConstructionScript`
  (`StaticMeshComponent.SetStaticMesh` (`self.StaticMesh`) (`|GetArrayItem` (`self.StationMeshes`) (`KismetMathLibrary.RandomInteger` 3))))