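; Time is a Blueprint function set that turns a float time in seconds into a display string of minutes, seconds and hundredths.
; TimeFormatMsms splits the value with truncation, modulo and fraction, takes absolute values so the sign is dropped, and joins the parts with colons.
; FormatDigit pads each part below ten with a leading zero.
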(fn `Format Digit`
  (params (String :type String))
  (returns (ReturnValue :type String))
  (return (select `bool` (< (`KismetStringLibrary.Conv_StringToInt` String) 10) :`false` String :`true` (`KismetStringLibrary.Concat_StrStr` "0" String))))

(fn `Time Format M-s-ms`
  (params (`Float time` :type "Float (double-precision)"))
  (returns (`Formated time` :type String))
  (bind _returnvalue (`KismetMathLibrary.FTrunc` `Float time`))
  (return (`KismetStringLibrary.Concat_StrStr` (`self.Format Digit` (`KismetStringLibrary.Conv_IntToString` (`KismetMathLibrary.Abs_Int` (`KismetMathLibrary.FTrunc` (/ (`KismetMathLibrary.Conv_IntToDouble` _returnvalue) 60.0))))) ":" (`self.Format Digit` (`KismetStringLibrary.Conv_IntToString` (`KismetMathLibrary.Abs_Int` (mod _returnvalue 60)))) ":" (`self.Format Digit` (`KismetStringLibrary.Conv_IntToString` (`KismetMathLibrary.Abs_Int` (`KismetMathLibrary.FTrunc` (* 100 (`KismetMathLibrary.Fraction` `Float time`)))))))))